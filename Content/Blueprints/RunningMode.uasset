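; RunningMode is an early scaffold for stepping a Runner actor through species genomes, apparently for a genetic-algorithm runner.
; Construction sizes the species list to its maximum and caches the first actor of the runner class.
; BeginPlay loads the indexed species and its genome as current.
; Each Tick advances the gene step, but the gene lookup and Runner reference are unconnected, so no input reaches the runner.
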(event EventBeginPlay
  (CallFunction|NewSpecies))

(event EventTick
  (params (DeltaSeconds :type Float%20%28single-precision%29))
  (CallFunction|SendInput))

(fn ConstructionScript
  (Utilities|Array|Resize (Variables|Default|GetSpeciesList) (Variables|Default|GetSpeciesMax))
  (bind _outactors (Actor|GetAllActorsOfClass (Variables|Default|GetRunnerClass)))
  (Variables|Default|SetRunner (Utilities|Array|Get(acopy) _outactors)))

(fn NewSpecies
  (bind _specieslist (Variables|Default|GetSpeciesList))
  (bind _speciesindex (Variables|Default|GetSpeciesIndex))
  (bind _item (Utilities|Array|Get(acopy) _specieslist _speciesindex))
  (Variables|Default|SetCurrentSpecies _item)
  (Variables|Default|SetCurrentGenome (.Genome (Utilities|Struct|BreakSpecies _item)))
  (return))

(fn SendInput
  (Variables|Default|SetGeneStep (+ (Variables|Default|GetGeneStep) 1))
  (return))