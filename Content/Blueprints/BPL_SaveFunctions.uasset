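; Blueprint function library that manages save slots for a generation-based simulation with species lists.
; A "Master" slot holds the current generation number, which builds each generation's slot name; both use GenerationSaveFile.
; Helpers create or load generation files, read the previous generation's species, and save each step until a cap signals completion.
; SaveLastSpeciesList is unfinished: it only calls the load and never writes its Species input.
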(fn `Create Master Save`
  (returns (Master :type "/Game/Blueprints/GenerationSaveFile Object Reference"))
  (bind _returnvalue (`GameplayStatics.CreateSaveGameObject` "/Game/Blueprints/GenerationSaveFile.GenerationSaveFile_C"))
  (bind _asgeneration_save_file (cast `/Game/Blueprints/GenerationSaveFile` _returnvalue)
    (:`then`
      (set `/Game/Blueprints/GenerationSaveFile.Generation` 0 _asgeneration_save_file)
      (`GameplayStatics.SaveGameToSlot` _asgeneration_save_file "Master")
      (return _asgeneration_save_file))
    (:`CastFailed`
      (return null))))

(fn `Create New Generation File`
  (returns (NewParam :type "/Game/Blueprints/GenerationSaveFile Object Reference"))
  (bind _returnvalue (`GameplayStatics.CreateSaveGameObject` "/Game/Blueprints/GenerationSaveFile.GenerationSaveFile_C"))
  (bind _asgeneration_save_file (cast `/Game/Blueprints/GenerationSaveFile` _returnvalue)
    (:`then`
      (bind _filename (`self.GenerationFileName` -1))
      (bind _output_get (set `/Game/Blueprints/GenerationSaveFile.SlotName` _filename _asgeneration_save_file))
      (`GameplayStatics.SaveGameToSlot` _asgeneration_save_file _output_get)
      (return _asgeneration_save_file))
    (:`CastFailed`
      (`KismetSystemLibrary.PrintString` null "ERROR:  Couldn't create new generation save.")
      (return null))))

(fn `GenerationFileName`
  (params (Generation :type Integer))
  (returns (Filename :type String))
  (bind _generation (`self.Load Generation Number` null))
  (bind _returnvalue (`KismetMathLibrary.SelectInt` Generation _generation (>= Generation 0)))
  (return (`KismetStringLibrary.Concat_StrStr` "Gen" (`KismetMathLibrary.SelectString` "0" "" (< _returnvalue 9)) (`KismetStringLibrary.Conv_IntToString` _returnvalue) "Savefile")))

(fn `Get Current Generation`
  (returns (`Current Save File` :type "/Game/Blueprints/GenerationSaveFile Object Reference"))
  (bind _generation (`self.Load Generation Number` null))
  (bind _filename (`self.GenerationFileName` _generation))
  (bind _returnvalue (`GameplayStatics.LoadGameFromSlot` _filename))
  (`/Engine/EditorBlueprintResources/StandardMacros.IsValid` _returnvalue
    (:`Is Valid`
      (bind _asgeneration_save_file (cast `/Game/Blueprints/GenerationSaveFile` _returnvalue)
        (:`then`
          (return _asgeneration_save_file))
        (:`CastFailed`
          _)))
    (:`Is Not Valid`
      _))
  (return null))

(fn `Increase Generation`
  (bind _returnvalue (`GameplayStatics.LoadGameFromSlot` "Master"))
  (bind _asgeneration_save_file (cast `/Game/Blueprints/GenerationSaveFile` _returnvalue))
  (set `/Game/Blueprints/GenerationSaveFile.Step` 0 _asgeneration_save_file)
  (`/Engine/EditorBlueprintResources/StandardMacros.IncrementInt` (`/Game/Blueprints/GenerationSaveFile.Generation` _asgeneration_save_file)
    (:`  `
      (`GameplayStatics.SaveGameToSlot` _asgeneration_save_file "Master"))))

(fn `Load Generation Number`
  (returns (Generation :type Integer))
  (bind _returnvalue (`GameplayStatics.LoadGameFromSlot` "Master"))
  (`/Engine/EditorBlueprintResources/StandardMacros.IsValid` _returnvalue
    (:`Is Valid`
      (bind _asgeneration_save_file (cast `/Game/Blueprints/GenerationSaveFile` _returnvalue)
        (:`then`
          (return (`/Game/Blueprints/GenerationSaveFile.Generation` _asgeneration_save_file)))
        (:`CastFailed`
          _)))
    (:`Is Not Valid`
      _))
  (bind _master (`self.Create Master Save` null))
  (return (`/Game/Blueprints/GenerationSaveFile.Generation` _master)))

(fn `Load Last Species List`
  (returns (`Species List` :type "Array of /Game/Blueprints/Species Structure") (`Save File` :type "/Game/Blueprints/GenerationSaveFile Object Reference"))
  (bind _array (`|MakeArray` (struct) :!type "/Game/Blueprints/Species Structure"))
  (bind _generation (`self.Load Generation Number` null))
  (bind _returnvalue (- _generation 1))
  (if (>= _returnvalue 0)
    (bind _filename (`self.GenerationFileName` _returnvalue))
    (bind _returnvalue_2 (`GameplayStatics.LoadGameFromSlot` _filename))
    (`/Engine/EditorBlueprintResources/StandardMacros.IsValid` _returnvalue_2
      (:`Is Valid`
        (bind _asgeneration_save_file (cast `/Game/Blueprints/GenerationSaveFile` _returnvalue_2)
          (:`then`
            (return (`/Game/Blueprints/GenerationSaveFile.Species` _asgeneration_save_file) _asgeneration_save_file))
          (:`CastFailed`
            _)))
      (:`Is Not Valid`
        (bind _returnvalue_3 (`GameplayStatics.CreateSaveGameObject` "/Game/Blueprints/GenerationSaveFile.GenerationSaveFile_C"))
        (`GameplayStatics.SaveGameToSlot` _returnvalue_3 _filename)
        (bind _asgeneration_save_file_2 (cast `/Game/Blueprints/GenerationSaveFile` _returnvalue_3)
          (:`then`
            (return _array _asgeneration_save_file_2))
          (:`CastFailed`
            _)))))
  (return _array null) ; if this ever happens, it's bad
)

(fn `Save Generation After Step`
  (params (SaveFile :type "/Game/Blueprints/GenerationSaveFile Object Reference"))
  (returns (`Generation Complete` :type Boolean))
  (bind _step (`/Game/Blueprints/GenerationSaveFile.Step` SaveFile))
  (if (< _step 128)
    (`/Engine/EditorBlueprintResources/StandardMacros.IncrementInt` _step
      (:`  `
        (`GameplayStatics.SaveGameToSlot` SaveFile (`/Game/Blueprints/GenerationSaveFile.SlotName` SaveFile))
        (return false)))
    (else
      (return true))))

(fn `Save Last Species List`
  (params (Species :type "Array of /Game/Blueprints/Species Structure"))
  (`self.Load Last Species List` null))