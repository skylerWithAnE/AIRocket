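; Base course obstacle segment that builds two rows of instanced tiles, one above the other, with a randomly chosen pipe child actor.
; Construction also moves a handle past the last tile to mark the next spawn point.
; DestroySeq starts a timeline intended to drive DestroyPieces, which swaps the leading tile pair for damaged destructible components with randomized impulses, then restarts the timeline to crumble the segment progressively.
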(event EventDestroySeq
  (bind _desttimeline (Variables|Default|GetDestTimeline))
  (if (not (Audio|Components|Audio|IsPlaying _desttimeline))
    (Components|Timeline|PlayfromStart _desttimeline)))

(fn ConstructionScript
  (bind _pipes (Variables|Default|GetPipes))
  (CallFunction|AddTiles)
  (bind _returnvalue (AddComponent|AddChildActorComponent false))
  (ChildActorComponent|SetChildActorClass _returnvalue (Utilities|Array|Get(acopy) _pipes (Math|Random|RandomInteger (Utilities|Array|Length _pipes)))))

(fn AddTiles
  (bind _instancedstaticmesh (Variables|Default|GetInstancedStaticMesh))
  (Components|InstancedStaticMesh|ClearInstances _instancedstaticmesh)
  (for _index (range 1 (Variables|Default|GetTileCount))
    (Components|InstancedStaticMesh|AddInstance _instancedstaticmesh (Math|Conversions|ToTransform(Vector) (LocalVariables|GetTileLoc)))
    (Components|InstancedStaticMesh|AddInstance _instancedstaticmesh (Math|Conversions|ToTransform(Vector) (+ (LocalVariables|GetTileLoc) "0, 0,680.000000")))
    (LocalVariables|SetTileLoc (+ (LocalVariables|GetTileLoc) "240.000000, 0, 0")))
  (Transformation|SetRelativeLocation (Variables|Default|GetNextSpawnHandle) (+ (.Location (Math|Transform|BreakTransform (.OutInstanceTransform (Components|InstancedStaticMesh|GetInstanceTransform _instancedstaticmesh (- (Components|InstancedStaticMesh|GetInstanceCount _instancedstaticmesh) 1) false)))) "125.000000, 0, 0") false))

(fn DestroyPieces
  (bind _instancedstaticmesh (Variables|Default|GetInstancedStaticMesh))
  (if (>= (Components|InstancedStaticMesh|GetInstanceCount (Variables|Default|GetInstancedStaticMesh)) 2)
    (CallFunction|AddDestructible)
    (Class|InstancedStaticMeshComponent|RemoveInstance _instancedstaticmesh)
    (CallFunction|AddDestructible)
    (Class|InstancedStaticMeshComponent|RemoveInstance _instancedstaticmesh)
    (Components|Timeline|PlayfromStart (Variables|Default|GetDestTimeline))))

(fn AddDestructible
  (bind _returnvalue (AddComponent|AddDestructibleComponent true (.OutInstanceTransform (Components|InstancedStaticMesh|GetInstanceTransform (Variables|Default|GetInstancedStaticMesh) 0 true))))
  (Game|Damage|ApplyDamage _returnvalue 1e+02 (Transformation|GetWorldLocation _returnvalue) (Math|Vector|MakeVector 3.0 (Math|Random|RandomFloatinRange -3.0 3.0) (Math|Random|RandomFloatinRange -3.0 3.0)) 1e+04))