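; Course platform actor that Runner-interface actors can pass through and that can be shattered on demand.
; A Box trigger switches off the static mesh's collision when a Runner overlaps it and restores it when the overlap ends.
; DestroySeq hides the mesh and disables its collision, then spawns a destructible component at the mesh's relative transform and applies radius damage to break it apart.
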(event `self.ReceiveBeginPlay`)

(event `self.ReceiveActorBeginOverlap`
  (params (OtherActor :type "Actor Object Reference")))

(event `self.ReceiveTick`
  (params (DeltaSeconds :type "Float (single-precision)")))

(event `self.Box.OnComponentBeginOverlap`
  (params (OtherActor :type "Actor Object Reference") (OtherComp :type "PrimitiveComponent Object Reference") (OtherBodyIndex :type Integer) (bFromSweep :type Boolean) (SweepResult :type "HitResult Structure (by ref)"))
  (if (`KismetSystemLibrary.DoesImplementInterface` OtherActor "/Game/Blueprints/Character/Runner.Runner_C")
    (`PrimitiveComponent.SetCollisionEnabled` (`self.StaticMesh`) "NoCollision")))

(event `self.Box.OnComponentEndOverlap`
  (params (OtherActor :type "Actor Object Reference") (OtherComp :type "PrimitiveComponent Object Reference") (OtherBodyIndex :type Integer))
  (if (`KismetSystemLibrary.DoesImplementInterface` OtherActor "/Game/Blueprints/Character/Runner.Runner_C")
    (`PrimitiveComponent.SetCollisionEnabled` (`self.StaticMesh`) "QueryAndPhysics")))

(event `/Game/Blueprints/Course/Hazards/OnscreenDestruction.DestroySeq`
  (bind _staticmesh (`self.StaticMesh`))
  (`SceneComponent.SetVisibility` _staticmesh false false)
  (`PrimitiveComponent.SetCollisionEnabled` _staticmesh "NoCollision")
  (bind _returnvalue (`AddComponent|Destructible Component_1823` :`RelativeTransform` (`SceneComponent.GetRelativeTransform` _staticmesh)))
  (`DestructibleComponent.ApplyRadiusDamage` _returnvalue 1.0 (`SceneComponent.K2_GetComponentLocation` _returnvalue) 360.0 300.0 true))

(fn `UserConstructionScript`)