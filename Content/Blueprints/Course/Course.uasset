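; Endless course manager that recycles a fixed set of CoursePiece actors into a continuous track along X.
; The construction script gathers all pieces in the level, attaches them and spaces them evenly, and BeginPlay randomizes obstacles beyond the first three.
; Passed events queue pieces after a short delay.
; Once more than two are queued, Tick teleports some to the tail with re-randomized obstacles, removing them from the queue mid-loop.
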(event EventTick
  (params (DeltaSeconds :type Float%20%28single-precision%29))
  (CallFunction|AddNewPiecesasNecessary))

(event Custom|Passed_Event_0
  (params (Passed%20Piece :type Course%20Piece%20Object%20Reference))
  (Utilities|FlowControl|Delay 1.0)
  (Variables|Default|SetPassCount (+ (Variables|Default|GetPassCount) 1))
  (Utilities|Array|Add (Variables|Default|GetAvailable%20Pieces) Passed%20Piece))

(event EventBeginPlay
  (for (_array_element _array_index) (Variables|Default|GetCourse%20Pieces)
    (EventDispatchers|AssignPassed _array_element (delegate Custom|Passed_Event_0))
    (if (> _array_index 2)
      (Default|RandomizeObstaclePiece _array_element))))

(fn ConstructionScript
  (bind _outactors (Actor|GetAllActorsOfClass "/Game/Blueprints/Course/CoursePiece.CoursePiece_C"))
  (bind _output_get (Variables|Default|SetCourse%20Pieces _outactors))
  (for _array_element _output_get
    (Class|Actor|AttachRootComponenttoActor _array_element self "None" "SnapToTarget" true)
    (Transformation|SetActorRelativeLocation _array_element (LocalVariables|GetCurrLoc))
    (bind _output_get_2 (LocalVariables|SetCurrLoc (+ (LocalVariables|GetCurrLoc) (Math|Vector|MakeVector 1.92e+03 0.0 0.0)))))
  (Variables|Default|SetCurrentSpawnLocation _output_get_2))

(fn AddNewPiecesasNecessary
  (bind _available_pieces (Variables|Default|GetAvailable%20Pieces))
  (bind _returnvalue (Utilities|Array|Length _available_pieces))
  (if (> _returnvalue 2)
    (bind (_array_element _array_index) (Utilities|Array|ForEachLoopwithBreak _available_pieces :!label _label)
      (:LoopBody
        (if (== _array_index (- _returnvalue 1))
          (goto _label Break)
          (else
            (CallFunction|MovePiecetoTail _array_element)
            (Utilities|Array|RemoveItem _available_pieces _array_element))))
      (:Completed
        (return)))
    (else
      (return))))

(fn MovePiecetoTail
  (params (Course%20Piece :type Course%20Piece%20Object%20Reference))
  (Transformation|Teleport Course%20Piece (Variables|Default|GetCurrentSpawnLocation) "0, 0, 0")
  (Default|RandomizeObstaclePiece Course%20Piece)
  (Variables|Default|SetCurrentSpawnLocation (+ (Variables|Default|GetCurrentSpawnLocation) (Math|Vector|MakeVector 1.92e+03 0.0 0.0))))