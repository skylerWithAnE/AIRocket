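; CoursePiece is one segment of a running course that hosts an obstacle and signals when the runner has passed it.
; When a RunningCharacter stops overlapping ExitCheckpoint, it fires Passed with itself as the argument.
; RandomizeObstaclePiece destroys the old obstacle component and actor, then spawns a random obstacle class, or the override in AIDemo, at its transform.
; CurrentPiece is then set to None, and the child-actor sizing logic is unconnected.
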(event `self.ReceiveBeginPlay`)

(event `self.ReceiveActorBeginOverlap`
  (params (OtherActor :type "Actor Object Reference")))

(event `self.ReceiveTick`
  (params (DeltaSeconds :type "Float (single-precision)")))

(event `self.ExitCheckpoint.OnComponentEndOverlap`
  (params (OtherActor :type "Actor Object Reference") (OtherComp :type "PrimitiveComponent Object Reference") (OtherBodyIndex :type Integer))
  (cast `/Game/Blueprints/Character/RunningCharacter` OtherActor)
  (`self.Passed` self))

(fn `RandomizeObstaclePiece`
  (params (`Class Override` :type "/Game/Blueprints/Course/ObstacleParent Class Reference"))
  (bind _currentpiece (`self.CurrentPiece`))
  (bind _obstpattern (`self.ObstPattern`))
  (bind _obstacleclasses (`self.ObstacleClasses`))
  (`/Engine/EditorBlueprintResources/StandardMacros.IsValid` _obstpattern
    (:`Is Valid`
      (`ActorComponent.K2_DestroyComponent` _obstpattern))
    (:`Is Not Valid`
      _))
  (`/Engine/EditorBlueprintResources/StandardMacros.IsValid` _currentpiece
    (:`Is Valid`
      (`self.K2_DestroyActor` _currentpiece))
    (:`Is Not Valid`
      _))
  (`|SpawnActorFromClass` (select `bool` (`self.AI Demo`) :`false` (`KismetArrayLibrary.Array_Get` _obstacleclasses (`KismetMathLibrary.RandomInteger` (`KismetArrayLibrary.Array_Length` _obstacleclasses))) :`true` `Class Override` :!type "Actor Class Reference") (`self.GetTransform`) "AlwaysSpawn" "OverrideRootScale")
  (set `self.CurrentPiece` null))

(fn `UserConstructionScript`)