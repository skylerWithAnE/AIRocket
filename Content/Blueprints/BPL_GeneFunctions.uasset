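; Blueprint function library for a genetic algorithm that evolves species whose genomes are sequences of Jump/Roll boolean genes.
; GetMostFit bubble-sorts by descending fitness, also swapping near-equal neighbors, and takes the top entries.
; MateAll pairs the first half of the parents with the second, producing fixed-size broods.
; Combine merges each gene pair by random AND/OR per action, occasionally mutating one by flipping it.
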(fn CompareSpecies
  (params (Species%201 :type Species%20Structure) (Species%202 :type Species%20Structure))
  (bind _fitness (Utilities|Struct|BreakSpecies Species%201))
  (bind _fitness_2 (Utilities|Struct|BreakSpecies Species%202))
  (return (Math|Integer|SelectInt 0 1 (and (not (Math|Float|NearlyEqual(Float) _fitness _fitness_2 0.001)) (> _fitness _fitness_2)))))

(fn SortAllSpecies
  (params (Input%20Array :type Array%20of%20Species%20Structures))
  (while (LocalVariables|GetSorting)
    (for _index (range 0 (- (Utilities|Array|Length Input%20Array) 2))
      (bind _result (CallFunction|CompareSpecies (Utilities|Array|Get(acopy) Input%20Array _index) (Utilities|Array|Get(acopy) Input%20Array (+ _index 1))))
      (if (== _result 1)
        (bind _output_get (LocalVariables|SetTemp (Utilities|Array|Get(acopy) Input%20Array _index)))
        (Utilities|Array|SetArrayElem Input%20Array _index (Utilities|Array|Get(acopy) Input%20Array (+ _index 1)))
        (Utilities|Array|SetArrayElem Input%20Array (+ _index 1) _output_get)
        (LocalVariables|SetSwapOccurred true)))
    (if (LocalVariables|GetSwapOccurred)
      (LocalVariables|SetSwapOccurred false)
      (else
        (LocalVariables|SetSorting false)))))

(fn IsGreaterThan
  (params (Species1 :type Species%20Structure) (Species2 :type Species%20Structure))
  (return (> (.Fitness (Utilities|Struct|BreakSpecies Species1)) (.Fitness (Utilities|Struct|BreakSpecies Species2)))))

(fn GetMostFit
  (params (InputArray :type Array%20of%20Species%20Structures) (SelectNum :type Integer))
  (CallFunction|SortAllSpecies InputArray)
  (for _index (range 0 (- SelectNum 1))
    (Utilities|Array|Add (LocalVariables|GetMostFit) (Utilities|Array|Get(acopy) InputArray _index)))
  (return (LocalVariables|GetMostFit)))

(fn MateAll
  (params (Parents :type Array%20of%20Species%20Structures))
  (bind _returnvalue (Utilities|Array|Length Parents))
  (bind _returnvalue_2 (/ _returnvalue 2))
  (for _index (range 0 (- _returnvalue_2 1))
    (bind _newchildren (CallFunction|Mate (Utilities|Array|Get(acopy) Parents _index) (Utilities|Array|Get(acopy) Parents (+ _index _returnvalue_2)) 16))
    (Utilities|Array|AppendArray (LocalVariables|GetTempChildren) _newchildren))
  (return (LocalVariables|GetTempChildren)))

(fn Mate
  (params (Parent1 :type Species%20Structure) (Parent2 :type Species%20Structure) (NumChildren :type Integer))
  (bind _tempgenome (LocalVariables|GetTempGenome))
  (for _index (range 0 (- NumChildren 1))
    (for (_array_element _array_index) (.Genome (Utilities|Struct|BreakSpecies Parent1))
      (bind _newgene (CallFunction|Combine _array_element (Utilities|Array|Get(acopy) (.Genome (Utilities|Struct|BreakSpecies Parent2)) _array_index)))
      (Utilities|Array|Add (LocalVariables|GetTempGenome) _newgene))
    (Utilities|Array|Add (LocalVariables|GetChildren) (Utilities|Struct|MakeSpecies 128 _tempgenome 0.0))
    (Utilities|Array|Clear _tempgenome))
  (return (LocalVariables|GetChildren)))

(fn Combine
  (params (Gene1 :type Gene%20Structure) (Gene2 :type Gene%20Structure))
  (bind (_jump _roll) (Utilities|Struct|BreakGene Gene1))
  (bind (_jump_2 _roll_2) (Utilities|Struct|BreakGene Gene2))
  (if (Math|Random|RandomBool)
    (LocalVariables|SetNewJump (and _jump _jump_2))
    (else
      (LocalVariables|SetNewJump (or _jump _jump_2))))
  (if (Math|Random|RandomBool)
    (LocalVariables|SetNewRoll (and _roll _roll_2))
    (else
      (LocalVariables|SetNewRoll (or _roll _roll_2))))
  (if (== (Math|Random|RandomIntegerinRange 1 10) 7)
    (if (Math|Random|RandomBool)
      (LocalVariables|SetNewJump (not (LocalVariables|GetNewJump)))
      (else
        (LocalVariables|SetNewRoll (not (LocalVariables|GetNewRoll))))))
  (return (Utilities|Struct|MakeGene (LocalVariables|GetNewJump) (LocalVariables|GetNewRoll))))