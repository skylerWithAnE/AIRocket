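; AC_Observer is a component that records the owning RunningCharacter's rocket and roll states as a gene sequence.
; Dispatcher events update the state flags, and a looping 0.1-second timer writes them as Jump/Roll genes into RecordedGene until its 128 slots are full.
; BeginPlay unbinds RollOn instead of binding it, so roll starts are not captured through that dispatcher.
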(event `self.ReceiveBeginPlay`
  (`KismetArrayLibrary.Array_Resize` (`self.RecordedGene`) 128)
  (`KismetSystemLibrary.K2_SetTimerDelegate` (delegate `Journal`) 0.1 true)
  (bind _asrunning_character (cast `/Game/Blueprints/Character/RunningCharacter` (`self.GetOwner`)))
  (bind _output_get (set `self.Rollbot` _asrunning_character))
  (add `/Game/Blueprints/Character/RunningCharacter.RocketOn` _output_get (delegate `RocketOn`))
  (add `/Game/Blueprints/Character/RunningCharacter.RocketOff` _output_get (delegate `RocketOff`))
  (remove `/Game/Blueprints/Character/RunningCharacter.RollOn` _output_get (delegate `RollOn`))
  (add `/Game/Blueprints/Character/RunningCharacter.RollOff` _output_get (delegate `RollOff`)))

(event `RocketOff`
  (set `self.Is Rocket On?` false))

(event `RollOff`
  (set `self.Is Roll On?` false))

(event `RollOn`
  (set `self.Is Roll On?` true))

(event `RocketOn`
  (set `self.Is Rocket On?` true))

(event `Journal`
  (bind _step (`self.Step`))
  (if (< _step 128)
    (`self.Journal Step`)
    (`/Engine/EditorBlueprintResources/StandardMacros.IncrementInt` _step)))

(fn `Journal Step`
  (`KismetArrayLibrary.Array_Set` (`self.RecordedGene`) (`self.Step`) (make `/Game/Blueprints/Gene` (`self.Is Rocket On?`) (`self.Is Roll On?`)))
  (return))