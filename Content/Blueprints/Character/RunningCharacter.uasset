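; Side-scrolling runner character that constantly moves along X, with jetpack, roll, jump and air dash, driven by input or AI events.
; Tick pans the background material, counters spring arm height and applies thrust through a gate, which rolling (crouch) blocks.
; Rocket while crouched jumps or air-dashes on cooldown; MoveDown boosts gravity, and WallRoll eases crouched characters toward a target.
; ExplodeAndDie detaches the camera, spawns explosions and calls Died.
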(event `self.ReceiveBeginPlay`
  (bind _returnvalue (`PrimitiveComponent.CreateDynamicMaterialInstance` (`self.BG`) 0 "/Game/HazardAssets/BG.BG"))
  (set `self.BGMat` _returnvalue))

(event `Rolling`
  (bind _returnvalue (`self.K2_GetActorLocation`))
  (bind _rolltolocation (`self.RollToLocation`))
  ;[1 1 1] this is disabled. and crap.
  (`/Engine/EditorBlueprintResources/StandardMacros.Gate` true :!via `Open` :!label _label
    (:`Exit`
      (if (== _returnvalue _rolltolocation :`ErrorTolerance` 10.0)
        (set `self.RollScalar` 1.0)
        (goto _label :!via `Close`)
        (else
          (`self.K2_SetActorLocation` (`KismetMathLibrary.VInterpTo` _returnvalue _rolltolocation (`GameplayStatics.GetWorldDeltaSeconds`) 60.0)))))))

(event `InputAxis|MoveDown`
  (params (AxisValue :type "Float (single-precision)"))
  (bind _charactermovement (`self.CharacterMovement`))
  (if (< AxisValue 0.0)
    (set `CharacterMovementComponent.GravityScale` 6.0 _charactermovement)
    (else
      (set `CharacterMovementComponent.GravityScale` 1.0 _charactermovement))))

(event `self.ReceiveTick`
  (params (DeltaSeconds :type "Float (single-precision)"))
  (bind _returnvalue (`self.GetInputAxisValue`))
  (bind _jetpackaudio (`self.JetpackAudio`))
  (bind _returnvalue_2 (`KismetMathLibrary.SelectFloat` 0.1 1.0 (< _returnvalue 0.0)))
  (`self.AddMovementInput` (1.0 0.0 0.0) (`KismetMathLibrary.SelectFloat` (+ _returnvalue _returnvalue_2) _returnvalue_2 (> _returnvalue 0.0)))
  (`|ExecutionSequence`
    (:`then_0`
      (`self.Pan Background`))
    (:`then_1`
      (`SceneComponent.K2_SetRelativeLocation` (`self.SpringArm`) (`KismetMathLibrary.MakeVector` 0.0 0.0 (- 250.0 (- (.z (`self.K2_GetActorLocation`)) 92.0))) false false))
    (:`then_2`
      (`/Engine/EditorBlueprintResources/StandardMacros.Gate` true :!label _label_2
        (:`Exit`
          (`CharacterMovementComponent.AddImpulse` (`self.CharacterMovement`) (* (`self.GetActorUpVector`) 5000.0) false)
          (`ActorComponent.Activate` (`self.JetFlames`) false)
          (if (not (`AudioComponent.IsPlaying` _jetpackaudio))
            (`AudioComponent.FadeIn` _jetpackaudio 0.5 1.0 0.0)))))))

(event `AIRocketOn`
  (`self.Try Jump` :!label _label_3)
  (`/Engine/EditorBlueprintResources/StandardMacros.Gate` false :!label _label_4
    (:`Exit`
      (goto _label_2 :!via `Open`))))

(event `InputAction|Rocket`
  (params (Key :type "Key Structure" :default "AnyKey"))
  (bind _charactermovement (`self.CharacterMovement`))
  (:`Pressed`
    (goto _label_3))
  (:`Released`
    (set `MovementComponent.Velocity` (`KismetMathLibrary.MakeVector` (.x (`MovementComponent.Velocity` _charactermovement)) 0.0 (.z (`MovementComponent.Velocity` _charactermovement))) _charactermovement :!label _label_5)
    (`ActorComponent.Deactivate` (`self.JetFlames`) :!label _label_6)
    (`AudioComponent.FadeOut` (`self.JetpackAudio`) 0.5 0.0)
    (goto _label_2 :!via `Close`)))

(event `AIRocketOff`
  (goto _label_5))

(event `AIRollOn`
  (`self.Crouch` :!label _label_7)
  (`|ExecutionSequence`
    (:`then_0`
      (goto _label_4 :!via `Close`))
    (:`then_1`
      (goto _label_6))))

(event `InputAction|Roll`
  (params (Key :type "Key Structure" :default "AnyKey"))
  (:`Pressed`
    (goto _label_7))
  (:`Released`
    (`self.UnCrouch` :!label _label_8)
    (goto _label_4 :!via `Open`)))

(event `AIRollOff`
  (goto _label_8))

(event `/Game/Blueprints/Character/Runner.WallRoll`
  (params (NewParam :type "Vector Structure"))
  (if (`NavMovementComponent.IsCrouching` (`self.CharacterMovement`))
    (set `self.InSweetSpot` true)
    (if (not (`TimelineComponent.IsPlaying` (`self.WallRollTimeline`)))
      (`Timeline|WallRollTimeline` :!via `PlayFromStart` :!label _label_9
        (:`Update`
          (`self.K2_SetActorLocation` (`KismetMathLibrary.VInterpTo` (`self.K2_GetActorLocation`) NewParam (`GameplayStatics.GetWorldDeltaSeconds`) 2.0)))))
    (else
      (set `self.InSweetSpot` false)
      (goto _label_9 :!via `Stop`))))

(event `/Game/Blueprints/Character/Runner.EndWallRoll`
  (set `self.InSweetSpot` false)
  (goto _label_9 :!via `Stop`))

(event `self.ReceiveAnyDamage`
  (params (Damage :type "Float (single-precision)") (DamageType :type "DamageType Object Reference") (InstigatedBy :type "Controller Object Reference") (DamageCauser :type "Actor Object Reference")))

(event `AirDashCoolDown`
  (set `self.AirDashAvailable` false)
  (`KismetSystemLibrary.Delay` 1.0)
  (set `self.AirDashAvailable` true))

(fn `CrouchMesh`)

(fn `Explode and Die`
  (bind _mesh (`self.Mesh`))
  (`/Engine/EditorBlueprintResources/StandardMacros.DoOnce` (`self.Dead`)
    (:`Completed`
      (`SceneComponent.DetachFromParent` (`self.Camera`) true true)
      (set `self.Dead` true)
      (`GameplayStatics.SpawnSoundAttached` "/Game/Audio/ExplodeCue.ExplodeCue" _mesh)
      (`SceneComponent.SetVisibility` _mesh false false)
      (`self.SetActorTickEnabled` false)
      (for _ (range 11)
        (`GameplayStatics.SpawnEmitterAtLocation` "/Game/StarterContent/Particles/P_Explosion.P_Explosion" (`self.K2_GetActorLocation`))
        (`self.Died`)))))

(fn `Pan Background`
  (bind _returnvalue (`KismetMathLibrary.VSize` (`KismetMathLibrary.MakeVector` (.x (`self.GetVelocity`)))))
  (bind _output_get (set `self.BGPanValue` (+ (`self.BGPanValue`) (`KismetMathLibrary.FClamp` (`KismetMathLibrary.SelectFloat` _returnvalue 0.0 (and (> _returnvalue 50.0) (not (`self.Dead`)))) 0.0 0.009))))
  (`MaterialInstanceDynamic.SetScalarParameterValue` (`self.BGMat`) "Pan" _output_get))

(fn `RollThroughObstacle`
  (params (Location :type "Vector Structure")))

(fn `Try Jump`
  (bind _jetpackaudio (`self.JetpackAudio`))
  (bind _charactermovement (`self.CharacterMovement`))
  (bind _charactermovement_2 (`self.CharacterMovement`))
  (bind _returnvalue (`NavMovementComponent.IsFalling` _charactermovement))
  (bind _returnvalue_2 (`NavMovementComponent.IsCrouching` _charactermovement))
  (if (and _returnvalue_2 (not _returnvalue))
    (`CharacterMovementComponent.AddImpulse` _charactermovement_2 (* (`self.GetActorUpVector`) 700.0) true)
    (`GameplayStatics.SpawnSoundAttached` "/Game/Audio/roll.roll" _jetpackaudio)
    (elif (and (`self.AirDashAvailable`) _returnvalue _returnvalue_2)
      (`CharacterMovementComponent.AddImpulse` _charactermovement_2 (* (`self.GetActorForwardVector`) 300.0) true)
      (`GameplayStatics.SpawnSoundAttached` "/Game/Audio/roll.roll" _jetpackaudio)
      (`self.AirDashCoolDown`)))
  (return))

(fn `UserConstructionScript`)