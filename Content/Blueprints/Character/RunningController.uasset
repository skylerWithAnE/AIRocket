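; Player controller for the Rollbot runner, handling HUD, pause and restart, plus an experimental genetic autopilot.
; Two save slots persist music position, which resumes across runs, and a species pool.
; Death or Backslash appends the observer's recorded genome with zero fitness, saves and restarts; Backslash also toggles autopilot.
; Autopilot steps through genes on a looping timer, driving rocket and roll from a randomly re-picked species at each lookup.
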(event `self.ReceiveBeginPlay`
  (bind _savesong (`self.savesong`))
  (`|ExecutionSequence`
    (:`then_0`
      (bind _returnvalue (`GameplayStatics.LoadGameFromSlot` (`self.Species Slotname`)))
      (`/Engine/EditorBlueprintResources/StandardMacros.IsValid` _returnvalue
        (:`Is Valid`
          (`KismetSystemLibrary.PrintString` "Loaded a species")
          (bind _newparam (`self.Cast to Species Save and Set` _returnvalue)
            (:`exec`
              (set `self.Run by Genetics?` (`/Game/Blueprints/SpeciesSave.Reset Helper` _newparam)))))
        (:`Is Not Valid`
          (`KismetSystemLibrary.PrintString` "Created a species")
          (bind _returnvalue_2 (`GameplayStatics.CreateSaveGameObject` "/Game/Blueprints/SpeciesSave.SpeciesSave_C"))
          (`self.Cast to Species Save and Set` _returnvalue_2))))
    (:`then_1`
      (bind _asrunning_character (cast `/Game/Blueprints/Character/RunningCharacter` (`self.K2_GetPawn`)))
      (set `self.Rollbot` _asrunning_character)
      (bind _returnvalue_3 (`GameplayStatics.LoadGameFromSlot` "main"))
      (`/Engine/EditorBlueprintResources/StandardMacros.IsValid` _returnvalue_3
        (:`Is Valid`
          (bind _assavefile (cast `/Game/Blueprints/Character/Savefile` _returnvalue_3))
          (bind _output_get (set `self.savesong` _assavefile)))
        (:`Is Not Valid`
          (bind _returnvalue_4 (`GameplayStatics.CreateSaveGameObject` "/Game/Blueprints/Character/Savefile.Savefile_C"))
          (bind _assavefile_2 (cast `/Game/Blueprints/Character/Savefile` _returnvalue_4))
          (set `self.savesong` _assavefile_2)))
      (`AudioComponent.Play` (`self.Audio`) (`/Game/Blueprints/Character/Savefile.Songtime` _output_get))
      (`|ExecutionSequence`
        (:`then_0`
          (bind (_direction _newtrack_0) (`Timeline|Timeline_0` :!via `PlayFromStart`)
            (:`Update`
              (if (`KismetMathLibrary.NearlyEqual_FloatFloat` _newtrack_0 1.0 0.01)
                (set `/Game/Blueprints/Character/Savefile.Songtime` (+ (`/Game/Blueprints/Character/Savefile.Songtime` _savesong) 1.0) _savesong)))))
        (:`then_1`
          (bind _returnvalue_5 (`|CreateWidget` "/Game/Blueprints/HUD/IngameHUD.IngameHUD_C"))
          (`UserWidget.AddToViewport` _returnvalue_5 0)
          (set `self.HUD` _returnvalue_5)
          (bind _asrunning_character_2 (cast `/Game/Blueprints/Character/RunningCharacter` (`GameplayStatics.GetPlayerPawn` 0)))
          (add `/Game/Blueprints/Character/RunningCharacter.Died` _asrunning_character_2 (delegate `Die`))
          (if (`self.Run by Genetics?`)
            (`KismetSystemLibrary.K2_SetTimerDelegate` (delegate `RunSpecies`) 0.1 true)))))))

(event `RunSpecies`
  (bind _gene_step (`self.Gene Step`))
  (bind _rollbot (`self.Rollbot`))
  (bind _species (`/Game/Blueprints/SpeciesSave.Species` (`self.SaveSpecies`)))
  (bind (_genomesize _genome) (break `/Game/Blueprints/Species` (`KismetArrayLibrary.Array_Get` _species (`KismetMathLibrary.RandomInteger` (`KismetArrayLibrary.Array_Length` _species)))))
  (bind (_jump _roll) (break `/Game/Blueprints/Gene` (`KismetArrayLibrary.Array_Get` _genome _gene_step)))
  (if (< _gene_step (`KismetArrayLibrary.Array_Length` _genome))
    (`|ExecutionSequence`
      (:`then_0`
        (if _jump
          (`/Game/Blueprints/Character/RunningCharacter.AIRocketOn` _rollbot)
          (else
            (`/Game/Blueprints/Character/RunningCharacter.AIRocketOff` _rollbot))))
      (:`then_1`
        (if _roll
          (`/Game/Blueprints/Character/RunningCharacter.AIRollOn` _rollbot)
          (else
            (`/Game/Blueprints/Character/RunningCharacter.AIRollOff` _rollbot))))
      (:`then_2`
        (`/Engine/EditorBlueprintResources/StandardMacros.IncrementInt` _gene_step)))))

(event `Key|Delete`
  (params (Key :type "Key Structure" :default "AnyKey"))
  (:`Pressed`
    (bind _returnvalue (`GameplayStatics.DeleteGameInSlot` (`self.Species Slotname`)))
    (`KismetSystemLibrary.PrintString` (`KismetStringLibrary.Conv_BoolToString` _returnvalue))
    (`KismetArrayLibrary.Array_Clear` (`/Game/Blueprints/SpeciesSave.Species` (`self.SaveSpecies`)))))

(event `Key|Backslash`
  (params (Key :type "Key Structure" :default "AnyKey"))
  (bind _savespecies (`self.SaveSpecies`))
  (bind _savesong (`self.savesong`))
  (:`Pressed`
    (set `/Game/Blueprints/SpeciesSave.Reset Helper` (not (`self.Run by Genetics?`)) _savespecies)
    (`KismetArrayLibrary.Array_Add` (`/Game/Blueprints/SpeciesSave.Species` _savespecies) (make `/Game/Blueprints/Species` 128 (`/Game/Blueprints/AC_Observer.RecordedGene` (`/Game/Blueprints/Character/RunningCharacter.AC_Observer` (`self.Rollbot`)))) :!label _label)
    (set `/Game/Blueprints/Character/Savefile.Songtime` (+ (`/Game/Blueprints/Character/Savefile.Songtime` _savesong) (`KismetSystemLibrary.GetGameTimeInSeconds`)) _savesong)
    (`GameplayStatics.SaveGameToSlot` _savesong "main")
    (`GameplayStatics.SaveGameToSlot` _savespecies (`self.Species Slotname`))
    (`KismetSystemLibrary.ExecuteConsoleCommand` "RestartLevel")))

(event `Key|Gamepad_RightShoulder` :paused true
  (params (Key :type "Key Structure" :default "AnyKey"))
  (bind _savesong (`self.savesong`))
  (:`Pressed`
    (if (and (`GameplayStatics.IsGamePaused`) (`self.IsInputKeyDown` "Gamepad_LeftShoulder"))
      (set `/Game/Blueprints/Character/Savefile.Songtime` 0.0 _savesong)
      (`GameplayStatics.SaveGameToSlot` _savesong "main")
      (`KismetSystemLibrary.ExecuteConsoleCommand` "Quit"))))

(event `Die`
  (`KismetSystemLibrary.Delay` 3.0)
  (goto _label))

(event `InputAction|Pause` :paused true
  (params (Key :type "Key Structure" :default "AnyKey"))
  (bind _pausecanvas (`/Game/Blueprints/HUD/IngameHUD.PauseCanvas` (`self.HUD`)))
  (:`Pressed`
    (if (`GameplayStatics.IsGamePaused`)
      (`Widget.SetVisibility` _pausecanvas "Hidden")
      (`GameplayStatics.SetGamePaused` false)
      (set `self.bShowMouseCursor` false)
      (else
        (`Widget.SetVisibility` _pausecanvas "Visible")
        (`GameplayStatics.SetGamePaused` true)
        (set `self.bShowMouseCursor` true)))))

(event `Key|Gamepad_FaceButton_Top` :paused true
  (params (Key :type "Key Structure" :default "AnyKey"))
  (:`Pressed`
    (if (`GameplayStatics.IsGamePaused`)
      (`GameplayStatics.SaveGameToSlot` (`self.savesong`) "main")
      (`KismetSystemLibrary.ExecuteConsoleCommand` "RestartLevel"))))

(event `self.Audio.OnAudioFinished`
  (bind _timeline_0 (`self.Timeline_0`))
  (`TimelineComponent.Stop` _timeline_0)
  (`AudioComponent.Play` (`self.Audio`) 0.0)
  (set `/Game/Blueprints/Character/Savefile.Songtime` 0.0 (`self.savesong`))
  (`TimelineComponent.PlayFromStart` _timeline_0))

(fn `UserConstructionScript`)